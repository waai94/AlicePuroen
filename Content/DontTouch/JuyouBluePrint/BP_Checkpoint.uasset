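; Checkpoint actor that records a save point the first time the player overlaps its box.
; On overlap it looks up a flag indexed by its checkpoint number plus a fixed offset.
; If unset, it passes its location to the save call, shows a saved-notification widget and sets the flag through the game mode.
; BeginPlay logs a warning for negative checkpoint numbers.
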(event OnComponentBeginOverlap(Box)
  (params (OverlappedComponent :type Primitive%20Component%20Object%20Reference) (OtherActor :type Actor%20Object%20Reference) (OtherComp :type Primitive%20Component%20Object%20Reference) (OtherBodyIndex :type Integer) (bFromSweep :type Boolean) (SweepResult :type Hit%20Result%20Structure%20%28by%20ref%29))
  (Utilities|Casting|CastToplayer OtherActor)
  (bind _flag (CallFunction|Getfag (+ (Variables|Default|GetCheckpointNum) 126)))
  (if (not _flag)
    (CallFunction|CheckpointSaved (Transformation|GetActorLocation))
    (bind _returnvalue (UserInterface|CreateWidget "/Game/DontTouch/System/Widget/Ensyutu/Checkpointsaved.Checkpointsaved_C"))
    (UserInterface|Viewport|AddtoViewport _returnvalue 0)
    (Class|Message|Setflagsate(Message) (Game|GetGameMode) true (+ (Variables|Default|GetCheckpointNum) 126))))

(event EventBeginPlay
  (if (< (Variables|Default|GetCheckpointNum) 0)
    (CallFunction|Printlog "CheckPointNumがx<0のものがあります！" "NewEnumerator4" true 2.0 false "(R=0.000000,G=1.000000,B=0.956444,A=1.000000)" "" "" "" false)))

(event Collision|EventActorBeginOverlap
  (params (OtherActor :type Actor%20Object%20Reference)))

(event EventTick
  (params (DeltaSeconds :type Float%20%28single-precision%29)))

(fn ConstructionScript)