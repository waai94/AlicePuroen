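; BP_Glass is a breakable glass actor that shatters as soon as play begins.
; On BeginPlay it spawns an FS_MasterField at its location, sets the radial magnitude and sphere radius, and triggers it, presumably fracturing the GlassBreakGeometryCollection.
; It then attaches a ManyTriagnelBurst particle effect to that collection.
; Delayed-trigger and field-cleanup nodes are disconnected, so the spawned field is never destroyed here.
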(event EventBeginPlay
  (bind _returnvalue (Game|SpawnActorfromClass "/Engine/EditorResources/FieldNodes/FS_MasterField.FS_MasterField_C" (Math|Transform|MakeTransform (Transformation|GetActorLocation)) "AlwaysSpawn" 0 0))
  (Variables|/Engine/EditorResources/FieldNodes/FS_MasterField.FS_MasterField_C|SetRadial%20Magnitude _returnvalue 5e+01)
  (Components|Sphere|SetSphereRadius (Variables|/Engine/EditorResources/FieldNodes/FS_MasterField.FS_MasterField_C|GetSphereVolumeCol _returnvalue) 4e+02 true)
  (Default|CETrigger _returnvalue)
  (Niagara|SpawnSystemAttached "/Game/DontTouch/Effect/ManyTriagnelBurst.ManyTriagnelBurst" (Variables|Default|GetGlassBreak_GeometryCollection) "None" "0, 0, 0" "0, 0, 0" "KeepRelativeOffset" false))

(event Collision|EventActorBeginOverlap
  (params (OtherActor :type Actor%20Object%20Reference)))

(event EventTick
  (params (DeltaSeconds :type Float%20%28single-precision%29)))

(fn ConstructionScript)