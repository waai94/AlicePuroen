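; Base event manager actor that runs step-by-step dialogue events, started when a testactor overlaps its Box.
; Talk hands message focus to itself via the player controller and replaces the current Messagewindow with one showing text, speaker, animation and choices (Sentakushi).
; NextPressed, unless a choice is pending, closes the window, increments Talknum and calls Gameevent, an empty hook apparently meant for child Blueprints.
; Tokusyu sets Talknum to jump between steps.
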(event OnComponentBeginOverlap(Box)
  (params (OverlappedComponent :type Primitive%20Component%20Object%20Reference) (OtherActor :type Actor%20Object%20Reference) (OtherComp :type Primitive%20Component%20Object%20Reference) (OtherBodyIndex :type Integer) (bFromSweep :type Boolean) (SweepResult :type Hit%20Result%20Structure%20%28by%20ref%29))
  (Utilities|Casting|CastTotestactor OtherActor)
  (CallFunction|Gameevent))

(event Custom|talk
  (params (text :type Text) (talker :type Text) (anim :type textanim%20Enum :default "NewEnumerator0") (sentakushi :type Array%20of%20Strings))
  (Variables|Default|Setisquestion (not (Utilities|Enum|Equal(Enum) (Utilities|Array|Get(acopy) sentakushi) "")))
  (Class|Message|Setnewfocus(Message) (Game|GetPlayerController 0) self)
  (Utilities|IsValid (Variables|Default|Getmywidget)
    (:Is%20Valid
      (Widget|RemovefromParent (Variables|Default|Getmywidget)))
    (:Is%20Not%20Valid
      _))
  (bind _returnvalue (UserInterface|CreateWidget "/Game/DontTouch/System/Widget/System/messagewindow.messagewindow_C" 0 (Utilities|String|ToString(Text) text) anim (Utilities|String|ToString(Text) talker) sentakushi))
  (Variables|Default|Setmywidget _returnvalue)
  (UserInterface|Viewport|AddtoViewport _returnvalue 0))

(event Custom|gameevent)

(event EventBeginPlay)

(event EventTick
  (params (DeltaSeconds :type Float%20%28single-precision%29)))

(event EventNextPressed
  (bind _mywidget (Variables|Default|Getmywidget))
  (if (not (Variables|Default|Getisquestion))
    (Utilities|IsValid _mywidget
      (:Is%20Valid
        (Widget|RemovefromParent _mywidget))
      (:Is%20Not%20Valid
        _))
    (Variables|Default|Settalknum (+ (Variables|Default|Gettalknum) 1))
    (CallFunction|Gameevent)))

(fn ConstructionScript)

(fn Tokusyu
  (params (index :type Integer))
  (Variables|Default|Settalknum (- index 1)))