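; Game system Blueprint that writes stage flags to the game instance and sanity-checks the level setup at start.
; Setflagsate sets one entry of the instance's Flag array by index, but always logs entry 1.
; BeginPlay resets the flags, then logs a problem if no StageManager exists or its StageName is empty.
; Tick is empty, and the delayed Reverse toggles are disconnected.
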(event EventBeginPlay
  (bind _asinstance (Utilities|Casting|CastToinstance (Game|GetGameInstance)))
  (Default|Resetflag _asinstance)
  (bind _returnvalue (Actor|GetActorOfClass "/Game/DontTouch/JuyouBluePrint/StageManager.StageManager_C"))
  (Utilities|IsValid _returnvalue
    (:Is%20Valid
      (if (Utilities|Enum|Equal(Enum) (Variables|/Game/DontTouch/JuyouBluePrint/StageManager.StageManager_C|GetStageName _returnvalue) (Utilities|Text|MakeLiteralText ""))
        (CallFunction|Printlog "StageName is null." "NewEnumerator2" true 2.0 false "(R=0.000000,G=1.000000,B=0.956444,A=1.000000)")))
    (:Is%20Not%20Valid
      (CallFunction|Printlog "StageManager is not Found!" "NewEnumerator4" true 2.0 false "(R=0.000000,G=1.000000,B=0.956444,A=1.000000)"))))

(event EventTick
  (params (DeltaSeconds :type Float%20%28single-precision%29)))

(event EventSetflagsate
  (params (checked :type Boolean) (index :type Integer))
  (bind _asinstance (Utilities|Casting|CastToinstance (Game|GetGameInstance))
    (:then
      (Utilities|Array|SetArrayElem (Variables|/Game/DontTouch/System/BluePrint/GameSystem/instance.instance_C|Getflag _asinstance) index checked)
      (CallFunction|Printlog (Utilities|String|ToString(Boolean) (Utilities|Array|Get(acopy) (Variables|/Game/DontTouch/System/BluePrint/GameSystem/instance.instance_C|Getflag _asinstance) 1)) "NewEnumerator1" true 2.0 false "(R=0.000000,G=1.000000,B=0.956444,A=1.000000)"))
    (:CastFailed
      (CallFunction|Printlog "failed" "NewEnumerator2" true 2.0 false "(R=0.000000,G=1.000000,B=0.956444,A=1.000000)"))))

(fn ConstructionScript)