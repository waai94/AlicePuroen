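; Game instance logic that manages progress flags, archive entries and the retry count.
; Resetflag rebuilds default and current flags from the Flags DataTable; ResetArchive reloads the Archive table, resets flags and calls SaveGame.
; Retry increments the count and calls SetArchive for separate entries at the first and fifth retries.
; SoftReset clears only flags marked Isreset, and only while the retry count is zero.
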(fn Resetflag
  (params (AllReset :type Boolean))
  (Utilities|Array|Clear (Variables|Default|GetDefualtFlag))
  (bind _outrownames (DataTable|GetDataTableRowNames "/Game/DontTouch/System/Construct/Flags.Flags"))
  (for _array_element _outrownames
    (bind _returnvalue (Utilities|GetDataTableRow "/Game/DontTouch/System/Construct/Flags.Flags" _array_element)
      (:then
        (Utilities|Array|Add (Variables|Default|GetDefualtFlag) _returnvalue))))
  (Utilities|Array|Clear (Variables|Default|GetNewFlag))
  (Variables|Default|SetNewFlag (Variables|Default|GetDefualtFlag)))

(fn ResetArchive
  (Utilities|Array|Clear (Variables|Default|GetArchive))
  (bind _outrownames (DataTable|GetDataTableRowNames "/Game/DontTouch/System/Construct/Archive.Archive"))
  (for _array_element _outrownames
    (bind _returnvalue (Utilities|GetDataTableRow "/Game/DontTouch/System/Construct/Archive.Archive" _array_element)
      (:then
        (Utilities|Array|Add (Variables|Default|GetArchive) _returnvalue))))
  (デフォルト|Resetflag false)
  (CallFunction|SaveGame))

(fn Retry
  (bind _result (Math|Integer|IncrementInt (Variables|Default|GetRetryNum))
    (:%20%20
      (if (== _result 1)
        (bind _returnvalue (CallFunction|SetArchive 5 1.0))
        (LocalVariables|SetNewLocalVar _returnvalue)
        (elif (== _result 5)
          (bind _returnvalue_2 (CallFunction|SetArchive 6 1.0))
          (LocalVariables|SetNewLocalVar _returnvalue_2)))
      (return (LocalVariables|GetNewLocalVar)))))

(fn SoftReset
  (bind _newflag (Variables|Default|GetNewFlag))
  (if (== (Variables|Default|GetRetryNum) 0)
    (for (_array_element _array_index) _newflag
      (Utilities|Array|SetArrayElem _newflag _array_index (Utilities|Struct|MakeFlagConstruct (and (.IsFlagSet (Utilities|Struct|BreakFlagConstruct _array_element)) (not (.Isreset (Utilities|Struct|BreakFlagConstruct _array_element)))) (.Isreset (Utilities|Struct|BreakFlagConstruct _array_element)) (.FlagName (Utilities|Struct|BreakFlagConstruct _array_element)))))))