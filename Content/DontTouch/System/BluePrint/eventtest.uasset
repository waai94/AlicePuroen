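; Test dialogue event that runs a scripted demo of the talk system's text display, with Japanese lines from an unnamed "???" speaker.
; Gameevent switches on Talknum to call Talk with text, animation and choices, using inline escape codes for color, size and other effects.
; Answered remaps Talknum at the two question steps, then re-runs Gameevent.
; Two branch lines also call Tokusyu with a later step number.
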(event EventBeginPlay
  (|CallParentFunction) ; このノードは無効になっているため呼び出せません。\n機能をビルドするにはピンをドラッグしてください。
)

(event EventGameevent
  (bind _array (Utilities|Array|MakeArray ""))
  (bind _defualtquestion (Variables|Default|Getdefualtquestion))
  (switch int (Variables|Default|Gettalknum)
    (:0
      (CallFunction|Talk "あー、あー、マイクテストマイクテスト" "???" "NewEnumerator0" (Utilities|Array|MakeArray "")))
    (:1
      (CallFunction|Talk "こんにちは！あなたは妖精ですか？" "???" "NewEnumerator2" (Utilities|Array|MakeArray "はい" "いいえ")))
    (:2
      (CallFunction|Talk "\\s5はえー" "???" "NewEnumerator3" _array)
      (CallFunction|Tokusyu 4))
    (:3
      (CallFunction|Talk "あなたは正直な人ですね。" "???" "NewEnumerator4" _array))
    (:4
      (CallFunction|Talk "まぁ、どうでもいいや。\\w2\\aここでは、文字の表示のテストをしています。" "???" "NewEnumerator2" _array))
    (:5
      (CallFunction|Talk "\\cr色\\を\\cy変えたり\\\\s4サイズ\\s2を\\s1変えたり" "???" "NewEnumerator0" _array))
    (:6
      (CallFunction|Talk "\\cg文字\\を揺らすこともできます。" "???" "NewEnumerator1" (Variables|Default|Getdefualtquestion)))
    (:7
      (CallFunction|Talk "さっきみたいに\\s4\\cp質問\\\\s2も付けることができます。" "???" "NewEnumerator4" (Utilities|Array|MakeArray "完璧に理解した" "そこそこ理解した" "なるほどわからん")))
    (:8
      (CallFunction|Talk "\\s5すごいですね" "???" "NewEnumerator3" _defualtquestion)
      (CallFunction|Tokusyu 10))
    (:9
      (CallFunction|Talk "これから頑張っていきましょう！\\s1\\w1ぶっちゃけ制作者も理解してないです" "???" "NewEnumerator0" _defualtquestion))
    (:10
      (CallFunction|Talk "以上でデモは終わりです！" "???" "NewEnumerator2" _defualtquestion))))

(event EventAnswered
  (params (answernum :type Integer))
  (Utilities|FlowControl|Sequence
    (:then_0
      (switch int (Variables|Default|Gettalknum)
        (:1
          (Variables|Default|Settalknum (Utilities|Select :Index answernum :Option%200 2 :Option%201 3)))
        (:7
          (Variables|Default|Settalknum (Utilities|Select :Index answernum :Option%200 8 :Option%201 9 :Option%202 9)))))
    (:then_1
      (CallFunction|Gameevent))))

(fn ConstructionScript
  (|CallParentFunction))