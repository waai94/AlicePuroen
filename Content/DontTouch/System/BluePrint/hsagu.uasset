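; An actor Blueprint that plays a one-time particle effect at its own location when its Gameevent event is triggered.
; Gameevent reads flag 0 and, if it is unset, spawns the Bbb system, then sets that flag through a message to the GameMode so later triggers do nothing.
; BeginPlay, overlap and Tick are unused placeholders, and the construction script only calls its parent.
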(event EventBeginPlay
  (|CallParentFunction) ; このノードは無効になっているため呼び出せません。\n機能をビルドするにはピンをドラッグしてください。
)

(event Collision|EventActorBeginOverlap
  (params (OtherActor :type Actor%20Object%20Reference)))

(event EventTick
  (params (DeltaSeconds :type Float%20%28single-precision%29))
  (|CallParentFunction DeltaSeconds) ; このノードは無効になっているため呼び出せません。\n機能をビルドするにはピンをドラッグしてください。
)

(event EventGameevent
  (bind _flag (CallFunction|Getfag))
  (if (not _flag)
    (Niagara|SpawnSystematLocation "/Game/DontTouch/IkalingChan/Effect/bbb.bbb" (Transformation|GetActorLocation))
    (Class|Message|Setflagsate(Message) (Game|GetGameMode) true)))

(fn ConstructionScript
  (|CallParentFunction))