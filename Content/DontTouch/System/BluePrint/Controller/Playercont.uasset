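; Player controller that handles global input for menus, messages and input-device detection.
; Tab opens a debug console outside distribution builds; the option action skips the player's active event or opens the pause menu, and jump advances the focused widget.
; Any key press writes keyboard/mouse or gamepad to a Material Parameter Collection, with axis keys (matched by Japanese display name "軸") filtered by a stick/look dead zone.
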(event Input|EnhancedActionEvents|EnhancedInputActionIA_option
  (params (ActionValue :type Vector%202D%20Structure) (ElapsedSeconds :type Float%20%28double-precision%29) (TriggeredSeconds :type Float%20%28double-precision%29) (InputAction :type Input%20Action%20Object%20Reference :default "/Game/DontTouch/System/Input/Actions/IA_option.IA_option"))
  (:Started
    (bind _asplayer (Utilities|Casting|CastToplayer (Game|GetPlayerCharacter 0))
      (:then
        (Utilities|IsValid (Variables|/Game/DontTouch/player.player_C|GetEventActor _asplayer)
          (:Is%20Valid
            (Class|Message|EventSkip(Message) (Variables|/Game/DontTouch/player.player_C|GetEventActor _asplayer))
            (Variables|/Game/DontTouch/player.player_C|SetEventActor _asplayer 0))
          (:Is%20Not%20Valid
            (bind _returnvalue (UserInterface|CreateWidget "/Game/DontTouch/System/Widget/Pause.Pause_C" :!label _label))
            (UserInterface|Viewport|AddtoViewport _returnvalue 0))))
      (:CastFailed
        (goto _label)))))

(event Input|EnhancedActionEvents|EnhancedInputActionIA_Jump
  (params (ActionValue :type Boolean) (ElapsedSeconds :type Float%20%28double-precision%29) (TriggeredSeconds :type Float%20%28double-precision%29) (InputAction :type Input%20Action%20Object%20Reference :default "/Game/DontTouch/System/Input/Actions/IA_Jump.IA_Jump"))
  (bind _focusedwidget (Variables|Default|GetFocusedWidget))
  (:Started
    (Utilities|IsValid _focusedwidget
      (:Is%20Valid
        (Class|Message|NextPressed(Message) _focusedwidget)))))

(event EventBeginPlay)

(event EventTick
  (params (DeltaSeconds :type Float%20%28single-precision%29)))

(event EventSetnewfocus
  (params (newactor :type Actor%20Object%20Reference))
  (Variables|Default|SetFocusedWidget newactor))

(event Input|KeyboardEvents|SpaceBar
  (params (Key :type Key%20Structure :default "None")))

(event Input|KeyboardEvents|Z
  (params (Key :type Key%20Structure :default "None")))

(event Input|KeyboardEvents|Tab
  (params (Key :type Key%20Structure :default "None"))
  (:Pressed
    (if (not (Class|KismetSystemLibrary|IsPackagedforDistribution))
      (bind _returnvalue (UserInterface|CreateWidget "/Game/DontTouch/System/Widget/System/Console.Console_C"))
      (UserInterface|Viewport|AddtoViewport _returnvalue 0))))

(event Input|KeyboardEvents|AnyKey
  (params (Key :type Key%20Structure :default "None"))
  (bind _returnvalue (Input|EnhancedActionValues|GetIA_Look))
  (bind _returnvalue_2 (Input|EnhancedActionValues|GetIA_Controller_Move))
  (bind _returnvalue_3 (Class|KismetMathLibrary|GetAbs2D _returnvalue))
  (bind _returnvalue_4 (Class|KismetMathLibrary|GetAbs2D _returnvalue_2))
  (bind (_x _y) (Math|Vector2D|BreakVector2D _returnvalue_3))
  (bind (_x_2 _y_2) (Math|Vector2D|BreakVector2D _returnvalue_4))
  (:Pressed
    (if (Utilities|String|Contains (Utilities|String|ToString(Text) (Class|KismetInputLibrary|KeyGetDisplayName Key true)) "軸")
      (if (Math|Boolean|ORBoolean (> _x_2 0.3) (> _y_2 0.3) (> _x 0.3) (> _y 0.3))
        (if (Class|KismetInputLibrary|KeyIsGamepadKey Key) :!label _label
          (Rendering|Material|SetScalarParameterValue "/Game/DontTouch/Material/Param/gamenchangeparam.gamenchangeparam" "InputDevice" 2.0 :!class /Script/Engine.KismetMaterialLibrary)
          (elif (Class|KismetInputLibrary|KeyIsKeyboardKey Key)
            (Rendering|Material|SetScalarParameterValue "/Game/DontTouch/Material/Param/gamenchangeparam.gamenchangeparam" "InputDevice" 1.0 :!class /Script/Engine.KismetMaterialLibrary :!label _label_2)
            (elif (Class|KismetInputLibrary|KeyIsMouseButton Key)
              (goto _label_2)))))
      (else
        (goto _label)))))

(fn ConstructionScript)