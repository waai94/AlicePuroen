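; Tutorial event actor that teaches the player to use an enemy to cross a gap too wide to jump.
; Gameevent shows Alice's hint dialogue and a button prompt for charge and boost on LB, then starts tutorial 9 after a short delay.
; The prompt widget is removed when the player leaves the Box trigger; nothing in this graph calls Gameevent.
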(event OnComponentEndOverlap(Box)
  (params (OverlappedComponent :type Primitive%20Component%20Object%20Reference) (OtherActor :type Actor%20Object%20Reference) (OtherComp :type Primitive%20Component%20Object%20Reference) (OtherBodyIndex :type Integer))
  (bind _newvar (Variables|Default|GetNewVar))
  (Utilities|Casting|CastToplayer OtherActor)
  (Utilities|IsValid _newvar
    (:Is%20Valid
      (Widget|RemovefromParent _newvar))))

(event EventBeginPlay
  (|CallParentFunction) ; このノードは無効になっているため呼び出せません。\n機能をビルドするにはピンをドラッグしてください。
)

(event Collision|EventActorBeginOverlap
  (params (OtherActor :type Actor%20Object%20Reference)))

(event EventTick
  (params (DeltaSeconds :type Float%20%28single-precision%29)))

(event EventGameevent
  (CallFunction|Talk "ここはジャンプでは飛び越えられなそうだ。あの敵を利用してみよう。" "Alice" "NewEnumerator0" (Utilities|Array|MakeArray "") 3.0 false)
  (bind _return (CallFunction|CreateTutorialButton (Utilities|Array|MakeArray (Utilities|Struct|MakeSousa "突進&加速" "/Game/DontTouch/Material/Buttons/ButtonLB.ButtonLB"))))
  (Variables|Default|SetNewVar _return)
  (Utilities|FlowControl|Delay 2.0)
  (CallFunction|Tutorial 9))

(fn ConstructionScript
  (|CallParentFunction))