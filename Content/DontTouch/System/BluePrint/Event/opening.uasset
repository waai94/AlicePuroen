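; Opening event that plays the Cheshire cat's dialogue with the player.
; camerachusi uses a timeline to turn the player's control rotation toward Chesa, then sets Talknum to 2 and runs Gameevent.
; Gameevent sets the character's event-message mode and switches on Talknum to show a line or end that mode.
; Answered branches Talknum on the chosen answer at step 2, then re-runs Gameevent.
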(event Custom|camerachusi
  (bind _returnvalue (Game|GetPlayerController 0))
  (Variables|Default|Setfirstrotate (Pawn|GetControlRotation _returnvalue :!class /Script/Engine.Controller))
  (bind _新規track_0 (Timeline|タイムライン PlayFromStart)
    (:Update
      (Pawn|SetControlRotation _returnvalue (Math|Rotator|Lerp(Rotator) (Variables|Default|Getfirstrotate) (Math|Rotator|FindLookatRotation (Transformation|GetActorLocation (Game|GetPlayerCharacter 0)) (Transformation|GetWorldLocation (Variables|Default|Getchesa))) _新規track_0 true)))
    (:Finished
      (Variables|Default|Settalknum 2)
      (CallFunction|Gameevent))))

(event EventBeginPlay
  (|CallParentFunction) ; このノードは無効になっているため呼び出せません。\n機能をビルドするにはピンをドラッグしてください。
)

(event Collision|EventActorBeginOverlap
  (params (OtherActor :type Actor%20Object%20Reference)))

(event EventTick
  (params (DeltaSeconds :type Float%20%28single-precision%29)))

(event EventGameevent
  (bind _returnvalue (Game|GetPlayerCharacter 0))
  (bind _defualtquestion (Variables|Default|Getdefualtquestion))
  (Class|Message|Seteventmode(Message) _returnvalue true)
  (switch int (Variables|Default|Gettalknum)
    (:0
      (CallFunction|Talk "下に降りてみなさい。\\cy双子\\が案内してくれるだろう・・・\\w1無事にいられるかわからないけどね。" "Cheshire cat" "NewEnumerator2" _defualtquestion 3.0 true :!label _label))
    (:1
      (Class|Message|Seteventmode(Message) _returnvalue false))
    (:2
      (CallFunction|Talk "こっちだにゃ。" "???" "NewEnumerator2" (Utilities|Array|MakeArray "") 3.0 true))
    (:3
      (CallFunction|Talk "この森に迷い込んでしまってるって顔をしているな。" "Cheshire cat" "NewEnumerator2" _defualtquestion 3.0 true))
    (:4
      (goto _label))))

(event EventAnswered
  (params (answernum :type Integer))
  (Utilities|FlowControl|Sequence
    (:then_0
      (switch string (Utilities|String|ToString(Integer) (Variables|Default|Gettalknum))
        (:2
          (Variables|Default|Settalknum (Utilities|Select :Index answernum :Option%200 3 :Option%201 4)))))
    (:then_1
      (CallFunction|Gameevent))))

(fn ConstructionScript
  (|CallParentFunction))