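; Base event actor for scripted dialogue, triggered when the player enters its box, either immediately or by taking controller focus to await a press.
; An empty Gameevent hook serves as the per-step script, keyed by Talknum, which NextPressed increments and Tokusyu redirects.
; Talk replaces the message window widget, optionally with choices that block NextPressed from advancing.
; Stopping lines take controller focus, while others auto-dismiss after a retriggerable delay.
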(event OnComponentBeginOverlap(Box)
  (params (OverlappedComponent :type Primitive%20Component%20Object%20Reference) (OtherActor :type Actor%20Object%20Reference) (OtherComp :type Primitive%20Component%20Object%20Reference) (OtherBodyIndex :type Integer) (bFromSweep :type Boolean) (SweepResult :type Hit%20Result%20Structure%20%28by%20ref%29))
  (bind _isneedpressed (Variables|Default|Getisneedpressed))
  (Utilities|Casting|CastToplayer OtherActor)
  (if (Variables|Default|GetIsDoOnce)
    (Utilities|FlowControl|DoOnce false
      (:Completed
        _)))
  (if _isneedpressed
    (Class|Message|Setnewfocus(Message) (Game|GetPlayerController 0) self)
    (if (not _isneedpressed)
      (Variables|Default|Settalknum 0 :!label _label)
      (CallFunction|Gameevent))
    (else
      (goto _label))))

(event OnComponentEndOverlap(Box)
  (params (OverlappedComponent :type Primitive%20Component%20Object%20Reference) (OtherActor :type Actor%20Object%20Reference) (OtherComp :type Primitive%20Component%20Object%20Reference) (OtherBodyIndex :type Integer))
  (Utilities|Casting|CastToplayer OtherActor)
  (Class|Message|Setnewfocus(Message) (Game|GetPlayerController 0)))

(event Custom|talk
  (params (text :type Text) (talker :type Text) (anim :type textanim%20Enum :default "NewEnumerator0") (sentakushi :type Array%20of%20Strings) (rotating :type Float%20%28double-precision%29) (withstop? :type Boolean))
  (Variables|Default|Setisquestion (not (Utilities|Enum|Equal(Enum) (Utilities|Array|Get(acopy) sentakushi) "")))
  (if withstop?
    (Class|Message|Setnewfocus(Message) (Game|GetPlayerController 0) self))
  (Utilities|IsValid (Variables|Default|Getmywidget)
    (:Is%20Valid
      (Widget|RemovefromParent (Variables|Default|Getmywidget)))
    (:Is%20Not%20Valid
      _))
  (bind _returnvalue (UserInterface|CreateWidget "/Game/DontTouch/System/Widget/System/messagewindow.messagewindow_C" 0 (Utilities|String|ToString(Text) text) anim (Utilities|String|ToString(Text) talker) sentakushi rotating "NewEnumerator2"))
  (Variables|Default|Setmywidget _returnvalue)
  (UserInterface|Viewport|AddtoViewport _returnvalue 0)
  (if (not withstop?)
    (Utilities|FlowControl|RetriggerableDelay 4.0)
    (Utilities|IsValid (Variables|Default|Getmywidget)
      (:Is%20Valid
        (Widget|RemovefromParent (Variables|Default|Getmywidget))))))

(event Custom|gameevent)

(event EventBeginPlay)

(event EventNextPressed
  (bind _mywidget (Variables|Default|Getmywidget))
  (Class|Message|Seteventmode(Message) (Game|GetPlayerCharacter 0) true)
  (if (not (Variables|Default|Getisquestion))
    (Utilities|IsValid _mywidget
      (:Is%20Valid
        (Widget|RemovefromParent _mywidget))
      (:Is%20Not%20Valid
        _))
    (Variables|Default|Settalknum (+ (Variables|Default|Gettalknum) 1))
    (CallFunction|Gameevent)))

(event EventSeteventmode
  (params (isevent :type Boolean))
  (Class|Message|Seteventmode(Message) (Game|GetPlayerCharacter 0) isevent))

(fn ConstructionScript)

(fn Tokusyu
  (params (index :type Integer))
  (Variables|Default|Settalknum (- index 1)))