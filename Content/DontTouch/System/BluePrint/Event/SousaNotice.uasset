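; SousaNotice is an event actor that shows a tutorial notice, apparently for controls ("sousa").
; Its Gameevent creates a TutorialButtonChild widget from the actor's text and material variables, adds it to the viewport and stores the reference.
; When the player stops overlapping the Box, it calls Delete on that widget if still valid.
; Nothing in this graph triggers Gameevent; the actor's own begin-overlap event is disabled.
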(event OnComponentEndOverlap(Box)
  (params (OverlappedComponent :type Primitive%20Component%20Object%20Reference) (OtherActor :type Actor%20Object%20Reference) (OtherComp :type Primitive%20Component%20Object%20Reference) (OtherBodyIndex :type Integer))
  (bind _newvar_0 (Variables|Default|GetNewVar_0))
  (Utilities|Casting|CastToplayer OtherActor)
  (Utilities|IsValid _newvar_0
    (:Is%20Valid
      (Default|Delete _newvar_0))))

(event EventBeginPlay
  (|CallParentFunction) ; このノードは無効になっているため呼び出せません。\n機能をビルドするにはピンをドラッグしてください。
)

(event Collision|EventActorBeginOverlap
  (params (OtherActor :type Actor%20Object%20Reference)))

(event EventTick
  (params (DeltaSeconds :type Float%20%28single-precision%29)))

(event EventGameevent
  (bind _returnvalue (UserInterface|CreateWidget "/Game/DontTouch/System/Widget/TutorialButtonChild.TutorialButtonChild_C" 0 (Variables|Default|GetSousaTextg) 0 (Variables|Default|GetMat)))
  (UserInterface|Viewport|AddtoViewport _returnvalue 0)
  (Variables|Default|SetNewVar_0 _returnvalue))

(fn ConstructionScript
  (|CallParentFunction))