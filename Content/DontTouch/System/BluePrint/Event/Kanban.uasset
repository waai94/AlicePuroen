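; Signboard (Kanban) event actor that shows a "落水に注意！" (beware of falling into water) warning as an announcer message.
; Gameevent logs Talknum and calls Talk with the default question set when it is zero.
; Any other value turns off the player character's event mode, then resets Talknum to -1 after a short delay.
; Talk is defined outside this graph, and nothing here advances Talknum.
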(event EventBeginPlay
  (|CallParentFunction) ; このノードは無効になっているため呼び出せません。\n機能をビルドするにはピンをドラッグしてください。
)

(event Collision|EventActorBeginOverlap
  (params (OtherActor :type Actor%20Object%20Reference)))

(event EventTick
  (params (DeltaSeconds :type Float%20%28single-precision%29)))

(event EventGameevent
  (CallFunction|Printlog (Utilities|String|ToString(Integer) (Variables|Default|Gettalknum)) "NewEnumerator0" true 2.0 false "(R=0.000000,G=1.000000,B=0.956444,A=1.000000)")
  (if (== (Variables|Default|Gettalknum) 0)
    (CallFunction|Talk "落水に注意！" "Announce" "NewEnumerator4" (Variables|Default|Getdefualtquestion) 2.0 true)
    (else
      (Class|Message|Seteventmode(Message) (Game|GetPlayerCharacter 0) false)
      (Utilities|FlowControl|Delay 0.2)
      (Variables|Default|Settalknum -1))))

(fn ConstructionScript
  (|CallParentFunction))