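; An event actor that offers the player a combat tutorial through a yes/no dialogue.
; Gameevent turns on the player character's event message mode and calls Talk with a System prompt asking whether to hear the battle explanation.
; Answered turns that mode off, moves the player to the TutorialBP actor's location on YES, then destroys this actor whatever the choice.
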(event EventBeginPlay
  (|CallParentFunction) ; このノードは無効になっているため呼び出せません。\n機能をビルドするにはピンをドラッグしてください。
)

(event Collision|EventActorBeginOverlap
  (params (OtherActor :type Actor%20Object%20Reference)))

(event EventTick
  (params (DeltaSeconds :type Float%20%28single-precision%29)))

(event EventGameevent
  (Class|Message|Seteventmode(Message) (Game|GetPlayerCharacter 0) true)
  (CallFunction|Talk "戦闘の説明をききますか？" "System" "NewEnumerator5" (Utilities|Array|MakeArray "YES" "NO") 0.0 true))

(event EventAnswered
  (params (answernum :type Integer))
  (Class|Message|Seteventmode(Message) (Game|GetPlayerCharacter 0) false)
  (if (== answernum 0)
    (bind _returnvalue (Actor|GetActorOfClass "/Game/DontTouch/System/BluePrint/Event/tutorialBP.tutorialBP_C"))
    (Transformation|SetActorLocation (Game|GetPlayerCharacter 0) (Transformation|GetActorLocation _returnvalue) false false))
  (Actor|DestroyActor))

(fn ConstructionScript
  (|CallParentFunction))