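; Tutorial event actor that teaches time stop at a river crossing where the footholds move too fast to board.
; Gameevent shows Alice's hint dialogue, creates a tutorial button prompt for stopping time, and calls ReduceTimePower with a large negative value, apparently to refill the player's time power.
; When the player leaves the Box volume, the stored prompt widget is removed from the screen.
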(event OnComponentEndOverlap(Box)
  (params (OverlappedComponent :type Primitive%20Component%20Object%20Reference) (OtherActor :type Actor%20Object%20Reference) (OtherComp :type Primitive%20Component%20Object%20Reference) (OtherBodyIndex :type Integer))
  (bind _return (Variables|Default|GetReturn))
  (Utilities|Casting|CastToplayer OtherActor)
  (Utilities|IsValid _return
    (:Is%20Valid
      (Widget|RemovefromParent _return))))

(event EventBeginPlay
  (|CallParentFunction) ; このノードは無効になっているため呼び出せません。\n機能をビルドするにはピンをドラッグしてください。
)

(event Collision|EventActorBeginOverlap
  (params (OtherActor :type Actor%20Object%20Reference)))

(event EventTick
  (params (DeltaSeconds :type Float%20%28single-precision%29)))

(event EventGameevent
  (CallFunction|Talk "川をわたりたいけど足場が速すぎて乗れない・・・。時を止めてみよう。" "Alice" "NewEnumerator5" (Utilities|Array|MakeArray "") 0.0 false)
  (bind _return (CallFunction|CreateTutorialButton (Utilities|Array|MakeArray (Utilities|Struct|MakeSousa "時を止める" "/Game/DontTouch/Material/Buttons/ButtonRT.ButtonRT"))))
  (Variables|Default|SetReturn _return)
  (bind _asplayer (Utilities|Casting|CastToplayer (Game|GetPlayerCharacter 0)))
  (Default|ReduceTimePower _asplayer -999.0 0.0))

(fn ConstructionScript
  (|CallParentFunction))