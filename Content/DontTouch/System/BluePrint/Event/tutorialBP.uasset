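; Tutorial director actor that teaches attacks, time rewind, acceleration and turret summoning through staged dialogue.
; Gameevent switches on Talknum into step graphs that play timed Talk lines, call Tutorial, show a control-hint widget and usually spawn a Boy target.
; The rewind step damages the player, advances itself, then comments based on HP.
; Out-of-order attack cases set Baka and rejoin the sequence; the final step moves the player to the Gotutorial actor.
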(event Custom|sousahyouzi
  (params (NewParam :type Text))
  (if (not (== (Utilities|String|Len (Utilities|String|ToString(Text) NewParam)) 0))
    (bind _returnvalue (UserInterface|CreateWidget "/Game/DontTouch/System/Widget/TUtorialButton.TUtorialButton_C" 0 NewParam))
    (UserInterface|Viewport|AddtoViewport _returnvalue 0)
    (Variables|Default|Setaa _returnvalue)))

(event EventBeginPlay
  (|CallParentFunction) ; このノードは無効になっているため呼び出せません。\n機能をビルドするにはピンをドラッグしてください。
)

(event Collision|EventActorBeginOverlap
  (params (OtherActor :type Actor%20Object%20Reference)))

(event EventTick
  (params (DeltaSeconds :type Float%20%28single-precision%29)))

(event EventGameevent
  (bind _array (Utilities|Array|MakeArray ""))
  (bind _array_2 (Utilities|Array|MakeArray ""))
  (bind _aa (Variables|Default|Getaa))
  (Utilities|IsValid _aa
    (:Is%20Valid
      (Default|Delete _aa))
    (:Is%20Not%20Valid
      _))
  (switch int (Variables|Default|Gettalknum)
    (:0
      (|0and1 _array _array _array :!label _label))
    (:1
      (goto _label execute2))
    (:2
      (|2))
    (:3
      (|3))
    (:4
      (|4))
    (:5
      (|5))
    (:6
      (CallFunction|Talk "よし！練習はここまでだ！" "???" "NewEnumerator2" (Utilities|Array|MakeArray "") 0.0 false)
      (Utilities|FlowControl|Delay (Variables|Default|GetDuration))
      (CallFunction|Talk "ここからはお前が道を切り開いてみせろ。" "???" "NewEnumerator2" (Utilities|Array|MakeArray "") 0.0 false)
      (bind _returnvalue (Actor|GetActorOfClass "/Game/DontTouch/System/BluePrint/Event/gotutorial.gotutorial_C"))
      (Utilities|IsValid _returnvalue
        (:Is%20Valid
          (Transformation|SetActorLocation (Game|GetPlayerCharacter 0) (Transformation|GetActorLocation _returnvalue) false false))))
    (:12
      (CallFunction|Talk "もうきょう攻撃を使っちゃうんだね！" "???" "NewEnumerator1" _array_2 0.0 false)
      (Utilities|FlowControl|Delay (Variables|Default|GetDuration))
      (Variables|Default|Settalknum 1)
      (Variables|Default|Setbaka true)
      (CallFunction|Gameevent))
    (:13
      (CallFunction|Talk "通常攻撃はさっき教えたでしょ。" "???" "NewEnumerator1" _array_2 0.0 false)
      (Utilities|FlowControl|Delay (Variables|Default|GetDuration))
      (Variables|Default|Settalknum 2)
      (Variables|Default|Setbaka true)
      (CallFunction|Gameevent))))

(fn ConstructionScript
  (|CallParentFunction))

(event Custom|spawn
  (Utilities|FlowControl|Delay 0.2)
  (CallFunction|Talk "今から出す的を倒してみろ。" "???" "NewEnumerator2" (Utilities|Array|MakeArray "") 2.0 false)
  (Utilities|FlowControl|Delay 3.0)
  (Game|SpawnActorfromClass "/Game/DontTouch/Enemies/boy.boy_C" (Math|Transform|MakeTransform (Transformation|GetActorLocation)) "AlwaysSpawn" 0 0 false 0)
  (CallFunction|Sousahyouzi (Variables|Default|Getmozi)))