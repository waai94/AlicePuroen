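; Global function library for flag lookups, achievement (Archive) unlocking and persistence, and a colored Niagara burst effect.
; Flags and achievements live in the game instance; SetArchive marks a first-time unlock, shows its popup widget and saves to slot 0.
; SaveGame and LoadGame copy only the achievement array to or from indexed slots, resetting it when no save loads.
; GetArchive only logs an achievement's name, description and unlock state.
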(fn Getfag
  (params (index :type Integer))
  (bind _asinstance (Utilities|Casting|CastToinstance (Game|GetGameInstance)))
  (return (Utilities|Array|Get(acopy) (Variables|/Game/DontTouch/System/BluePrint/GameSystem/instance.instance_C|Getflag _asinstance) index) index))

(fn SetArchive
  (params (Number :type Integer))
  (bind _asinstance (Utilities|Casting|CastToinstance (Game|GetGameInstance)))
  (if (not (.Obtain (Utilities|Struct|BreakAchiveConstruct (Utilities|Array|Get(acopy) (Variables|/Game/DontTouch/System/BluePrint/GameSystem/instance.instance_C|GetArchive _asinstance) Number))))
    (Utilities|Array|SetArrayElem (Variables|/Game/DontTouch/System/BluePrint/GameSystem/instance.instance_C|GetArchive _asinstance) Number (Utilities|Struct|MakeAchiveConstruct (.Name (Utilities|Struct|BreakAchiveConstruct (Utilities|Array|Get(acopy) (Variables|/Game/DontTouch/System/BluePrint/GameSystem/instance.instance_C|GetArchive _asinstance) Number))) true (.Setumei (Utilities|Struct|BreakAchiveConstruct (Utilities|Array|Get(acopy) (Variables|/Game/DontTouch/System/BluePrint/GameSystem/instance.instance_C|GetArchive _asinstance) Number))) (.Date (Utilities|Struct|BreakAchiveConstruct (Utilities|Array|Get(acopy) (Variables|/Game/DontTouch/System/BluePrint/GameSystem/instance.instance_C|GetArchive _asinstance) Number))) (.Serclet (Utilities|Struct|BreakAchiveConstruct (Utilities|Array|Get(acopy) (Variables|/Game/DontTouch/System/BluePrint/GameSystem/instance.instance_C|GetArchive _asinstance) Number)))))
    (bind _returnvalue (UserInterface|CreateWidget "/Game/DontTouch/System/Widget/ArchiveWidget.ArchiveWidget_C" 0 Number))
    (UserInterface|Viewport|AddtoViewport _returnvalue 0)
    (CallFunction|SaveGame)))

(fn SaveGame
  (params (Index :type Integer))
  (bind _returnvalue (Utilities|String|ToString(Integer) Index))
  (bind _returnvalue_2 (SaveGame|LoadGamefromSlot (Utilities|String|Append "GameSlot" _returnvalue)))
  (Utilities|IsValid _returnvalue_2
    (:Is%20Valid
      (bind _asbp_save_game (Utilities|Casting|CastToBP_SaveGame _returnvalue_2))
      (LocalVariables|SetSaveData _asbp_save_game)
      (bind _asinstance (Utilities|Casting|CastToinstance (Game|GetGameInstance))))
    (:Is%20Not%20Valid
      (bind _returnvalue_3 (SaveGame|CreateSaveGameObject "/Game/DontTouch/JuyouBluePrint/BP_SaveGame.BP_SaveGame_C"))
      (LocalVariables|SetSaveData _returnvalue_3)))
  (Variables|/Game/DontTouch/JuyouBluePrint/BP_SaveGame.BP_SaveGame_C|SetSavedArchive (LocalVariables|GetSaveData) (Variables|/Game/DontTouch/System/BluePrint/GameSystem/instance.instance_C|GetArchive _asinstance))
  (bind _returnvalue_4 (SaveGame|SaveGametoSlot (LocalVariables|GetSaveData) (Utilities|String|Append "GameSlot" _returnvalue)))
  (CallFunction|Printlog (Utilities|String|ToString(Boolean) _returnvalue_4) "NewEnumerator0" true 4.0 false "(R=0.000000,G=1.000000,B=0.956444,A=1.000000)" "" "Save: "))

(fn LoadGame
  (params (Index :type Integer))
  (bind _returnvalue (SaveGame|LoadGamefromSlot (Utilities|String|Append "GameSlot" (Utilities|String|ToString(Integer) Index))))
  (Utilities|IsValid _returnvalue
    (:Is%20Valid
      (bind _asbp_save_game (Utilities|Casting|CastToBP_SaveGame _returnvalue))
      (bind _asinstance (Utilities|Casting|CastToinstance (Game|GetGameInstance)))
      (Variables|/Game/DontTouch/System/BluePrint/GameSystem/instance.instance_C|SetArchive _asinstance (Variables|/Game/DontTouch/JuyouBluePrint/BP_SaveGame.BP_SaveGame_C|GetSavedArchive _asbp_save_game)))
    (:Is%20Not%20Valid
      (bind _asinstance_2 (Utilities|Casting|CastToinstance (Game|GetGameInstance)))
      (Default|ResetArchive _asinstance_2))))

(fn GetArchive
  (params (index :type Integer))
  (bind _asinstance (Utilities|Casting|CastToinstance (Game|GetGameInstance)))
  (CallFunction|Printlog (Utilities|String|Append "実績：" (Utilities|String|ToString(Text) (.Name (Utilities|Struct|BreakAchiveConstruct (Utilities|Array|Get(acopy) (Variables|/Game/DontTouch/System/BluePrint/GameSystem/instance.instance_C|GetArchive _asinstance) index)))) "," "説明（" (Utilities|String|ToString(Text) (.Setumei (Utilities|Struct|BreakAchiveConstruct (Utilities|Array|Get(acopy) (Variables|/Game/DontTouch/System/BluePrint/GameSystem/instance.instance_C|GetArchive _asinstance) index)))) ")" ".解除状況:" (Utilities|String|ToString(Boolean) (.Obtain (Utilities|Struct|BreakAchiveConstruct (Utilities|Array|Get(acopy) (Variables|/Game/DontTouch/System/BluePrint/GameSystem/instance.instance_C|GetArchive _asinstance) index))))) "NewEnumerator5" true 5.0 false "(R=0.000000,G=1.000000,B=0.956444,A=1.000000)"))

(fn SpawnTriangleBurst
  (params (Location :type Vector) (Color :type Vector :default "1.000000,1.000000,1.000000"))
  (bind _returnvalue (Niagara|SpawnSystematLocation 0 "/Game/DontTouch/Effect/TriangleBurst.TriangleBurst" Location))
  (Niagara|SetNiagaraVariable(Vector3) _returnvalue "Color" Color))