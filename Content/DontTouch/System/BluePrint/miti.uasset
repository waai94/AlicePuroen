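; Spline-based actor, apparently a path ("miti"), that builds collidable mesh geometry along its spline.
; The construction script aligns the spline to the scene root, then adds a Cube1 spline mesh component per segment with query and physics collision.
; Each mesh starts at point 0 rather than the segment's own start and ends at the next point, so meshes overlap.
; The event graph holds no active logic.
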(event EventBeginPlay)

(event Collision|EventActorBeginOverlap
  (params (OtherActor :type Actor%20Object%20Reference)))

(event EventTick
  (params (DeltaSeconds :type Float%20%28single-precision%29)))

(fn ConstructionScript
  (bind _spline (Variables|Default|GetSpline))
  (bind _spline_2 (Variables|Default|GetSpline))
  (bind (_location _tangent) (Spline|GetLocationandTangentatSplinePoint _spline_2 0 "Local"))
  (Transformation|SetWorldTransform _spline (Transformation|GetWorldTransform (Variables|Default|GetDefaultSceneRoot)) false false)
  (for _index (range 0 (- (Class|SplineComponent|GetNumberOfSplineSegments _spline) 1))
    (bind _returnvalue (AddComponent|AddSplineMeshComponent false))
    (Transformation|AttachComponentToComponent _returnvalue (Variables|Default|GetSpline) "None" "KeepRelative" "KeepRelative" "KeepRelative" true)
    (Components|StaticMesh|SetStaticMesh _returnvalue "/Engine/BasicShapes/Cube1.Cube1")
    (SplineMesh|SetStartandEnd _returnvalue _location _tangent (.Location (Spline|GetLocationandTangentatSplinePoint _spline_2 (+ _index 1) "Local")) (.Tangent (Spline|GetLocationandTangentatSplinePoint _spline_2 (+ _index 1) "Local")) true :!class /Script/Engine.SplineMeshComponent)
    (Collision|SetCollisionEnabled _returnvalue "QueryAndPhysics")))