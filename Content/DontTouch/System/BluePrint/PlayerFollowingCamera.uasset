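; Trigger-zone camera actor that takes over the view while the player is inside its Box and follows them in one of several modes.
; Every Tick, Followmode selects moving the SpringArm to the player, rotating the SpringArm toward them, or rotating only the Camera.
; Box overlaps blend the view to this camera and back to the player, logging the overlapping component.
; On exit, control rotation is matched to the camera's.
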(event OnComponentBeginOverlap(Box)
  (params (OverlappedComponent :type Primitive%20Component%20Object%20Reference) (OtherActor :type Actor%20Object%20Reference) (OtherComp :type Primitive%20Component%20Object%20Reference) (OtherBodyIndex :type Integer) (bFromSweep :type Boolean) (SweepResult :type Hit%20Result%20Structure%20%28by%20ref%29))
  (Utilities|Casting|CastToplayer OtherActor)
  (Game|Player|SetViewTargetwithBlend (Game|GetPlayerController 0) self 1.0 "VTBlend_EaseInOut" 3.0 false)
  (CallFunction|Printlog (Utilities|GetDisplayName OtherComp) "NewEnumerator0" true 2.0 false "(R=0.000000,G=1.000000,B=0.956444,A=1.000000)"))

(event OnComponentEndOverlap(Box)
  (params (OverlappedComponent :type Primitive%20Component%20Object%20Reference) (OtherActor :type Actor%20Object%20Reference) (OtherComp :type Primitive%20Component%20Object%20Reference) (OtherBodyIndex :type Integer))
  (bind _asplayer (Utilities|Casting|CastToplayer OtherActor))
  (Game|Player|SetViewTargetwithBlend (Game|GetPlayerController 0) _asplayer 1.0 "VTBlend_EaseInOut" 3.0 false)
  (Pawn|SetControlRotation (Game|GetPlayerController 0) (Transformation|GetWorldRotation (Variables|Default|GetCamera)))
  (CallFunction|Printlog (Utilities|GetDisplayName OtherComp) "NewEnumerator0" true 2.0 false "(R=0.000000,G=1.000000,B=0.956444,A=1.000000)"))

(event EventBeginPlay)

(event Collision|EventActorBeginOverlap
  (params (OtherActor :type Actor%20Object%20Reference)))

(event EventTick
  (params (DeltaSeconds :type Float%20%28single-precision%29))
  (bind _returnvalue (Game|GetPlayerCharacter 0))
  (bind _springarm (Variables|Default|GetSpringArm))
  (bind _camera (Variables|Default|GetCamera))
  (bind _returnvalue_2 (Transformation|GetActorLocation _returnvalue))
  (switch int (Variables|Default|Getfollowmode)
    (:0
      (Transformation|SetWorldLocation _springarm _returnvalue_2 false false))
    (:1
      (Transformation|SetWorldRotation _springarm (Math|Rotator|FindLookatRotation (Transformation|GetWorldLocation _springarm) _returnvalue_2) false false))
    (:2
      (Transformation|SetWorldRotation _camera (Math|Rotator|FindLookatRotation (Transformation|GetWorldLocation _camera) _returnvalue_2) false false))))

(fn ConstructionScript)