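; A temporary effect light actor that shows a colored point light fading out over its lifetime.
; BeginPlay applies the configured color, sets the actor lifespan from Time, and unhides the light after the Affecttime delay.
; Tick counts Time down and linearly lerps intensity toward zero by the remaining fraction, so the fade already runs during that delay.
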(event EventBeginPlay
  (Rendering|Components|Light|SetLightColor (Variables|Default|GetPointLight) (Variables|Default|Getlightcolor) true)
  (Actor|SetLifeSpan (Variables|Default|Gettime))
  (Variables|Default|Setmaxtime (Variables|Default|Gettime))
  (Utilities|FlowControl|Delay (Variables|Default|Getaffecttime))
  (Development|SetHiddeninGame (Variables|Default|GetPointLight) false false))

(event Collision|EventActorBeginOverlap
  (params (OtherActor :type Actor%20Object%20Reference)))

(event EventTick
  (params (DeltaSeconds :type Float%20%28single-precision%29))
  (Rendering|Components|Light|SetIntensity (Variables|Default|GetPointLight) (Math|Float|Lerp 0.0 9308.0 (/ (Variables|Default|Gettime) (Variables|Default|Getmaxtime))))
  (Variables|Default|Settime (- (Variables|Default|Gettime) DeltaSeconds)))

(fn ConstructionScript)