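; BP_Weapon is a test weapon actor that plays a Genshin-style appear and glow effect one second after spawning.
; BeginPlay measures the weapon's length between its Top and Base sockets and passes it to dynamic material instances created for every skeletal mesh material.
; Two timelines then run together, driving appear-line and glow scalar parameters on those materials through a shared setter.
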(event Custom|StartGlowLine
  (bind _appeartrack (Timeline|GlowTimeLine Play)
    (:Update
      (CallFunction|SetWeaponAppearLine _appeartrack "GlowTimeLine"))))

(event Custom|StartAppearLine
  (bind _appeartrack (Timeline|AppearTimeline Play)
    (:Update
      (bind _output_get (Variables|Default|SetWeaponLine _appeartrack))
      (CallFunction|SetWeaponAppearLine _output_get "AppearLine"))))

(event EventBeginPlay
  (CallFunction|CalculateWeaponHeight)
  (for (_array_element _array_index) (Rendering|Material|GetMaterials (Variables|Default|GetSkeletalMesh))
    (bind _returnvalue (Rendering|Material|CreateDynamicMaterialInstance (Variables|Default|GetSkeletalMesh) _array_index _array_element "None" :!class /Script/Engine.PrimitiveComponent))
    (Utilities|Array|Add (Variables|Default|GetWeaponMaterial) _returnvalue)
    (Rendering|Material|SetScalarParameterValue _returnvalue "WeaponHeight" (Variables|Default|GetWeaponHeight) :!class /Script/Engine.MaterialInstanceDynamic))
  (CallFunction|SetWeaponAppearLine 0.0 "AppearLine")
  (Utilities|FlowControl|Delay 1.0)
  (CallFunction|StartAppearLine)
  (CallFunction|StartGlowLine))

(fn ConstructionScript)

(fn CalculateWeaponHeight
  (bind _skeletalmesh (Variables|Default|GetSkeletalMesh))
  ;[1 1 1] 仕込んだソケット間の距離を表示領域の長さとする
  (Variables|Default|SetWeaponHeight (Math|Vector|VectorLength (- (Transformation|GetSocketLocation _skeletalmesh "Top") (Transformation|GetSocketLocation _skeletalmesh "Base")))))

(fn SetWeaponAppearLine
  (params (AppearLine :type Float%20%28single-precision%29) (ParamName :type Name))
  (for _array_element (Variables|Default|GetWeaponMaterial)
    (Rendering|Material|SetScalarParameterValue _array_element ParamName AppearLine :!class /Script/Engine.MaterialInstanceDynamic)))