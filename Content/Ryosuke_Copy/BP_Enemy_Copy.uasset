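; Enemy character, optionally a boss that activates on sight, with melee attacks, time manipulation and ragdoll death.
; A spawned Reversingsystem records HP, velocity and time each tick, and receives time dilation and rewind requests.
; Hits during altered time are banked with stacking multipliers, then applied as one sum when time normalizes.
; Damage handling adds backstab and critical bonuses, while melee hits each overlapping player once per attack window.
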(event OnComponentBeginOverlap(Box)
  (params (OverlappedComponent :type Primitive%20Component%20Object%20Reference) (OtherActor :type Actor%20Object%20Reference) (OtherComp :type Primitive%20Component%20Object%20Reference) (OtherBodyIndex :type Integer) (bFromSweep :type Boolean) (SweepResult :type Hit%20Result%20Structure%20%28by%20ref%29)))

(event OnSeePawn(PawnSensing)
  (params (Pawn :type Pawn%20Object%20Reference))
  (if (Variables|Default|Getboss)
    (CallFunction|IamSeeing)))

(event Custom|talk
  (params (text :type Text) (talker :type Text) (anim :type textanim%20Enum :default "NewEnumerator0") (rotating :type Float%20%28double-precision%29))
  (Utilities|IsValid (Variables|Default|Getmywidget)
    (:Is%20Valid
      (Widget|RemovefromParent (Variables|Default|Getmywidget)))
    (:Is%20Not%20Valid
      _))
  (bind _returnvalue (UserInterface|CreateWidget "/Game/DontTouch/System/Widget/messagewindow.messagewindow_C" 0 (Utilities|String|ToString(Text) text) anim (Utilities|String|ToString(Text) talker) (Utilities|Array|MakeArray "") rotating "NewEnumerator2"))
  (Variables|Default|Setmywidget _returnvalue)
  (UserInterface|Viewport|AddtoViewport _returnvalue 0)
  (Utilities|FlowControl|Delay 5.0)
  (Utilities|IsValid (Variables|Default|Getmywidget)
    (:Is%20Valid
      (Widget|RemovefromParent (Variables|Default|Getmywidget)))))

(event Custom|attack
  (bind _mesh (Variables|Character|GetMesh))
  (bind _returnvalue (Components|SkeletalMesh|GetAnimInstance _mesh))
  ;[1 1 1] 攻撃系
  (Utilities|IsValid _mesh
    (:Is%20Valid
      (Utilities|IsValid _returnvalue
        (:Is%20Valid
          (if (not (Animation|Montage|MontageIsPlaying _returnvalue 0))
            (if (Variables|Default|Getcanwalk)
              (Animation|PlayAnimMontage (Variables|Default|GetNormalAttackMotion) 1.0 "None"))))))))

(event Custom|IamSeeing
  (Utilities|FlowControl|DoOnce false
    (:Completed
      (CallFunction|Start)
      (bind _returnvalue (UserInterface|CreateWidget "/Game/DontTouch/System/Widget/caution.caution_C" 0 false (Variables|Default|Getname) self true))
      (UserInterface|Viewport|AddtoViewport _returnvalue 0)
      (bind _returnvalue_2 (Actor|GetActorOfClass "/Game/DontTouch/System/BluePrint/GameSystem/audiomanager.audiomanager_C"))
      (Default|Audiochange _returnvalue_2 "/Game/DontTouch/sound/BGM/boss.boss"))))

(event Custom|re)

(event Custom|autoattack)

(event Custom|spawn
  (Actor|Tick|SetActorTickEnabled true)
  (Rendering|SetActorHiddenInGame false)
  (Collision|SetCollisionEnabled (Variables|Collision|GetCapsuleComponent) "QueryAndPhysics")
  (Collision|SetCollisionEnabled (Variables|Character|GetMesh) "QueryAndPhysics")
  (Class|Message|Logicstart(Message) (AI|GetAIController self) true)
  (CallFunction|Start))

(event Custom|start
  (Utilities|FlowControl|DoOnce false
    (:Completed
      (CallFunction|Spawn)
      (bind _returnvalue (Game|SpawnActorfromClass "/Game/DontTouch/JuyouBluePrint/reversingsystem.reversingsystem_C" (Transformation|GetActorTransform) "AlwaysSpawn" 0 0 self false 0))
      (Variables|Default|Setreverseactor _returnvalue)
      (Utilities|FlowControl|Delay 0.0)
      (Niagara|SpawnSystematLocation "/Game/DontTouch/Effect/spawn.spawn" (Transformation|GetActorLocation))
      (Utilities|FlowControl|Delay 0.3)
      (bind _returnvalue_2 (Niagara|SpawnSystematLocation "/Game/DontTouch/Effect/hate.hate" (Transformation|GetActorLocation)))
      (Effects|Components|ParticleSystem|SetVectorParameter _returnvalue_2 "target" (Transformation|GetActorLocation (Game|GetPlayerCharacter 0)))
      (Utilities|FlowControl|Delay (Math|Random|RandomFloatinRange 1.0 4.0)))))

(event Custom|died
  (if (Variables|Default|Getboss)
    (bind _returnvalue (UserInterface|CreateWidget "/Game/DontTouch/System/Widget/compelte.compelte_C" 0 999.0))
    (UserInterface|Viewport|AddtoViewport _returnvalue 0)))

(event Custom|applytimedamage
  (if (Variables|Default|Gettimecontroled)
    (goto _label Reset)
    (else
      (Utilities|FlowControl|DoOnce false :!label _label
        (:Completed
          (bind _added1 (CallFunction|TasizanSuruKansuu))
          (Game|Damage|ApplyDamage self _added1 0 (Game|GetPlayerCharacter 0) "/Script/Engine.DamageType")
          (Utilities|Array|Clear (Variables|Default|Getsaveddamage)))))))

(event Custom|attackon
  ;[1 1 1] 攻撃系
  (Variables|Default|Setcanapplydamage true)
  (Utilities|Array|Clear (Variables|Default|Getattackedactor)))

(event Custom|attackoff
  ;[1 1 1] 攻撃系
  (Variables|Default|Setcanapplydamage false))

(event EventBeginPlay
  (Utilities|Time|SetTimerbyFunctionName 0 "applytimedamage" 0.05 true)
  (Variables|Default|SetHP (Variables|Default|Getmaxhp))
  (if (not (Variables|Default|Getboss))
    (CallFunction|Spawn)
    (bind _returnvalue (Game|SpawnActorfromClass "/Game/DontTouch/JuyouBluePrint/reversingsystem.reversingsystem_C" (Transformation|GetActorTransform) "AlwaysSpawn" 0 0 self false 0))
    (Variables|Default|Setreverseactor _returnvalue)
    (Utilities|FlowControl|Delay 0.0)
    (Niagara|SpawnSystematLocation "/Game/DontTouch/Effect/spawn.spawn" (Transformation|GetActorLocation))
    (Utilities|FlowControl|Delay 0.3)
    (bind _returnvalue_2 (Niagara|SpawnSystematLocation "/Game/DontTouch/Effect/hate.hate" (Transformation|GetActorLocation)))
    (Effects|Components|ParticleSystem|SetVectorParameter _returnvalue_2 "target" (Transformation|GetActorLocation (Game|GetPlayerCharacter 0)))
    (Utilities|FlowControl|Delay (Math|Random|RandomFloatinRange 1.0 4.0))))

(event Collision|EventActorBeginOverlap
  (params (OtherActor :type Actor%20Object%20Reference)))

(event EventTick
  (params (DeltaSeconds :type Float%20%28single-precision%29))
  (CallFunction|Timecontrol)
  (CallFunction|Stuncontrol)
  (CallFunction|Attackhantei))

(event EventSetnewcustomtime
  (params (dilution :type Float%20%28double-precision%29) (time :type Float%20%28double-precision%29) (isrewind :type Boolean))
  (bind _reverseactor (Variables|Default|Getreverseactor))
  (Utilities|IsValid _reverseactor
    (:Is%20Valid
      (Default|Settimedictiom _reverseactor dilution time isrewind))))

(event Game|Damage|EventPointDamage
  (params (Damage :type Float%20%28single-precision%29) (DamageType :type Damage%20Type%20Object%20Reference) (HitLocation :type Vector :default "0, 0, 0") (HitNormal :type Vector :default "0, 0, 0") (HitComponent :type Primitive%20Component%20Object%20Reference) (BoneName :type Name :default "None") (ShotFromDirection :type Vector :default "0, 0, 0") (InstigatedBy :type Controller%20Object%20Reference) (DamageCauser :type Actor%20Object%20Reference) (HitInfo :type Hit%20Result%20Structure%20%28by%20ref%29))
  (Variables|Default|Setimpact HitNormal))

(event EventHuttobasu
  (params (Vector :type Vector :default "0, 0, 0"))
  (bind _mesh (Variables|Character|GetMesh))
  (Physics|AddImpulse (Variables|Character|GetCharacterMovement) Vector true)
  (Utilities|FlowControl|Delay 0.05)
  (if (Physics|IsSimulatingPhysics _mesh "None")
    (Physics|AddImpulse _mesh Vector "None" true)))

(event EventReverseValue
  (params (HP :type Float%20%28double-precision%29) (Velocity :type Vector :default "0, 0, 0") (time :type Float%20%28double-precision%29))
  (Variables|Default|SetHP HP)
  (Variables|/Script/Engine.MovementComponent|SetVelocity (Variables|Character|GetCharacterMovement) Velocity)
  (Variables|Default|Setmytime time))

(event Game|Damage|EventAnyDamage
  (params (Damage :type Float%20%28single-precision%29) (DamageType :type Damage%20Type%20Object%20Reference) (InstigatedBy :type Controller%20Object%20Reference) (DamageCauser :type Actor%20Object%20Reference))
  (bind _returnvalue (Transformation|GetActorLocation))
  (bind _returnvalue_2 (Transformation|GetActorLocation DamageCauser))
  (bind _mesh (Variables|Character|GetMesh))
  (bind _reverseactor (Variables|Default|Getreverseactor))
  (bind _mycreatedspawner (Variables|Default|Getmycreatedspawner))
  (Variables|Default|Setdamagegain Damage)
  (Utilities|FlowControl|Sequence
    (:then_0
      (Utilities|IsValid DamageCauser
        (:Is%20Valid
          (CallFunction|Gotdamage _returnvalue_2)
          (if (<= (Variables|Default|GetHP) 0.0)
            (Utilities|FlowControl|DoOnce false
              (:Completed
                (CallFunction|Died)
                (Class|Message|Kyoukichange(Message) (Game|GetPlayerCharacter 0) (Math|Float|SelectFloat 4e+01 1.0 (Variables|Default|Getisally)))
                (Utilities|FlowControl|Delay 0.2)
                (Actor|Tick|SetActorTickEnabled false)
                (Physics|SetSimulatePhysics _mesh true)
                (Physics|AddImpulse _mesh (* (Variables|Default|Getimpact) -4000) "None" false)
                (Collision|SetCollisionEnabled (Variables|Collision|GetCapsuleComponent) "NoCollision")
                (Pawn|Components|CharacterMovement|SetMovementMode (Variables|Character|GetCharacterMovement) "MOVE_None" 0)
                (Utilities|FlowControl|Sequence
                  (:then_0
                    (Utilities|IsValid _reverseactor
                      (:Is%20Valid
                        (Actor|DestroyActor _reverseactor)
                        (bind _asai (Utilities|Casting|CastToai (Pawn|GetController))
                          (:then
                            (Default|Logicstart _asai false))
                          (:CastFailed
                            _)))
                      (:Is%20Not%20Valid
                        _))
                    (Utilities|FlowControl|Delay 1.0)
                    (Niagara|SpawnSystematLocation "/Game/DontTouch/Effect/death.death" (Transformation|GetSocketLocation (Variables|Character|GetMesh) "Spine_02"))
                    (Utilities|IsValid _mycreatedspawner
                      (:Is%20Valid
                        (Actor|DestroyActor _mycreatedspawner))
                      (:Is%20Not%20Valid
                        _))
                    (Actor|DestroyActor)))))))))
    (:then_1
      (Utilities|IsValid DamageCauser
        (:Is%20Valid
          (Niagara|SpawnSystematLocation "/Game/DontTouch/Effect/bisya.bisya" _returnvalue (Math|Rotator|FindLookatRotation _returnvalue_2 _returnvalue)))))
    (:then_2
      (if (== (Utilities|GetClass DamageType) "/Game/DontTouch/System/BluePrint/tokitome.tokitome_C")
        (Math|Integer|IncrementInt (Variables|Default|Getdamagecombo))))))

(event EventDestroyed
  (bind _myspawner (Variables|Default|Getmyspawner))
  (Utilities|IsValid _myspawner
    (:Is%20Valid
      (Default|Enemykilled _myspawner))))

(event EventGoingDamage
  (params (damage :type Float%20%28double-precision%29) (hitlocation :type Vector :default "0, 0, 0") (iroiro :type Boolean) (Cause :type Actor%20Object%20Reference) (DamageType :type Damage%20Type%20Class%20Reference) (DamageScore :type Float%20%28double-precision%29) (AdditonalEffect :type AdditionalEffect%20Enum :default "NewEnumerator3") (AdditionalEffectTime :type Float%20%28double-precision%29) (GoingStun :type Float%20%28double-precision%29))
  (|GoingDamaged damage damage Cause DamageType hitlocation))

(fn ConstructionScript)

(fn Gotgravit
  (if (not (AI|Components|NavMovement|IsFalling (Variables|Character|GetCharacterMovement)))
    (if (Variables|Default|Getgravit)
      (Game|Damage|ApplyDamage self 3e+02 0 0)
      (Variables|Default|Setgravit false))))

(fn Timecontrol
  (bind _customtimedilation (Variables|Default|GetCustomTimeDilation))
  (bind _reverseactor (Variables|Default|Getreverseactor))
  (bind _returnvalue (== _customtimedilation 1.0))
  (Utilities|FlowControl|Sequence
    (:then_0
      (Utilities|IsValid _reverseactor
        (:Is%20Valid
          (Default|Recordvalue _reverseactor (Variables|Default|GetHP) (Variables|/Script/Engine.MovementComponent|GetVelocity (Variables|Character|GetCharacterMovement)) false (Variables|Default|Getmytime))
          (Variables|Default|Settimecontroled (not _returnvalue))
          (Rendering|SetCustomDepthStencilValue (Variables|Character|GetMesh) (Math|Integer|SelectInt 1 3 _returnvalue))
          (if _returnvalue
            _))))
    (:then_1
      (Variables|Default|SetMutekiDamageTimer (- (Variables|Default|GetMutekiDamageTimer) (* (Utilities|Time|GetWorldDeltaSeconds) 6e+01))))))

(fn Stuncontrol
  (bind _output_get (Variables|Default|Setisstuned (>= (Variables|Default|Getstunparam) (Variables|Default|Getneedstun))))
  (Variables|/Script/Engine.CharacterMovementComponent|SetMaxWalkSpeed (Variables|Character|GetCharacterMovement) (Math|Float|SelectFloat (Variables|Default|Getwalkspeed) 0.0 (Variables|Default|Getcanwalk))))

(fn Moving)

(fn Gotdamage
  (params (NewParam :type Vector))
  (if (<= (Variables|Default|GetMutekiDamageTimer) 0.0)
    (if (< (Math|Vector|DotProduct (Math|Vector|Normalize (- NewParam (Transformation|GetActorLocation))) (Transformation|GetActorForwardVector)) -0.75)
      (Variables|Default|Setdamagegain (* (Variables|Default|Getdamagegain) 1.5)))
    (if (<= (Math|Random|RandomFloatinRange 0.0 1e+02) 5.0)
      (LocalVariables|Setcriticalhit true)
      (Variables|Default|Setdamagegain (* (Variables|Default|Getdamagegain) 2.0)))
    (bind _returnvalue (UserInterface|CreateWidget "/Game/DontTouch/System/Widget/damage.damage_C" 0 (Utilities|String|ToString(Integer) (Math|Float|Truncate (Variables|Default|Getdamagegain))) (LocalVariables|Getcriticalhit) (Math|Vector|SelectVector (Transformation|GetActorLocation) (Variables|Default|Getdaamgehitlocation) (Variables|Default|GetDamagetextOnEnemyActor))))
    (UserInterface|Viewport|AddtoViewport _returnvalue 0)
    (Variables|Default|SetHP (- (Variables|Default|GetHP) (Variables|Default|Getdamagegain)))))

(fn Attackhantei
  (bind _attackedactor (Variables|Default|Getattackedactor))
  (Utilities|FlowControl|Sequence
    (:then_0
      (if (Variables|Default|Getcanapplydamage)
        (for _array_element (Collision|GetOverlappingActors (Variables|Default|GetBox) "/Game/DontTouch/player.player_C" :!class /Script/Engine.PrimitiveComponent)
          (if (not (Utilities|Array|ContainsItem _attackedactor _array_element))
            (Game|Damage|ApplyDamage _array_element (Variables|Default|GetATK) 0 self)
            (Utilities|Array|Add _attackedactor _array_element)
            (CallFunction|Printlog (Utilities|GetDisplayName _array_element) "NewEnumerator0" true 2.0 false "(R=0.000000,G=1.000000,B=0.956444,A=1.000000)")))))))

(fn Spawnmyspawner
  (bind _returnvalue (Game|SpawnActorfromClass "/Game/DontTouch/JuyouBluePrint/SpawnerFold/spawner.spawner_C" (Transformation|GetActorTransform) "AlwaysSpawn" 0 false 0))
  (Variables|Default|Setmycreatedspawner _returnvalue)
  (Default|Onlyspawn _returnvalue))

(fn TasizanSuruKansuu
  (for _array_element (Variables|Default|Getsaveddamage)
    (LocalVariables|SetAdded (+ _array_element (LocalVariables|GetAdded))))
  (return (LocalVariables|GetAdded)))