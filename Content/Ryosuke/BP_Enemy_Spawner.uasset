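; Enemy spawner actor that spawns ten Torisan_2 enemies at random points inside its Box component when play begins.
; The Spawn event caches each spawn location in the Enemy array and the actor reference in Enemy2.
; An unconnected, unfinished boids-style separation pass compares those cached locations to accumulate a Y-axis separation vector, but it never runs.
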(event Custom|Spawn
  (bind _box (Variables|Default|GetBox))
  (bind (_origin _boxextent) (Collision|GetComponentBounds _box))
  (for _index (range 0 9)
    (bind _returnvalue (Game|SpawnActorfromClass "/Game/Ryosuke/torisan_2.torisan_2_C" (Math|Transform|MakeTransform (Math|Random|RandomPointinBoundingBox _origin _boxextent) "0, 0, 0" "1.000000,1.000000,1.000000") "Undefined" 0 0 0))
    (Utilities|Array|SetArrayElem (Variables|Default|GetEnemy) _index (.location (Transformation|GetActorTransform _returnvalue)) true)
    (Utilities|Array|SetArrayElem (Variables|Default|GetEnemy2) _index _returnvalue true)))

(event EventBeginPlay
  (CallFunction|Spawn))

(event Collision|EventActorBeginOverlap
  (params (OtherActor :type Actor%20Object%20Reference)))

(event EventTick
  (params (DeltaSeconds :type Float%20%28single-precision%29)))

(fn ConstructionScript)