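; Enemy character, optionally a boss with caution widget, music change and DPS-check phase.
; Tick drives montage attacks with box-overlap hits, walk control and timers; perception feeds the Blackboard.
; Damage applies backstab, critical and difficulty multipliers, then handles combo scoring and ragdoll death.
; A spawned Reversingsystem records state for rewind; hits during altered time dilation are stored with stacking bonuses, then applied together when time normalises.
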(event OnComponentBeginOverlap(Box)
  (params (OverlappedComponent :type Primitive%20Component%20Object%20Reference) (OtherActor :type Actor%20Object%20Reference) (OtherComp :type Primitive%20Component%20Object%20Reference) (OtherBodyIndex :type Integer) (bFromSweep :type Boolean) (SweepResult :type Hit%20Result%20Structure%20%28by%20ref%29))
  ;[1 1 1] プログラムまとめた
)

(event OnPerceptionUpdated(AIPerception)
  (params (UpdatedActors :type Array%20of%20Actor%20Object%20References))
  (for _array_element UpdatedActors
    (if (not (Variables|Default|Getfind))
      (if (== _array_element (Game|Player|GetPlayerPawn 0))
        (Variables|Default|Setfind true))))
  (AI|Components|Blackboard|SetValueasBool (AI|GetBlackboard (AI|GetAIController self)) (Utilities|Name|MakeLiteralName "Find") (Variables|Default|Getfind))
  (if (Variables|Default|Getfind)
    (Variables|Default|Setfind false)))

(event OnTargetPerceptionInfoUpdated(AIPerception)
  (params (UpdateInfo :type Actor%20Perception%20Update%20Info%20Structure%20%28by%20ref%29)))

(event Custom|re
  ;[1 1 1] プログラムまとめた
)

(event Custom|died
  ;[1 1 1] プログラムまとめた
  ;;[1 1 1] ボス用のプログラム
  (if (Variables|Default|Getboss)
    (Widget|RemovefromParent (Variables|Default|GetMyCaution))
    (Utilities|FlowControl|Delay 0.1)
    (Utilities|Time|SetGlobalTimeDilation 0.01)
    (Utilities|FlowControl|Delay 0.02)
    (Utilities|Time|SetGlobalTimeDilation 1.0)
    (bind _returnvalue (UserInterface|CreateWidget "/Game/DontTouch/System/Widget/System/FinalResult.FinalResult_C"))
    (UserInterface|Viewport|AddtoViewport _returnvalue 0)
    (bind _returnvalue_2 (Actor|GetActorOfClass "/Game/DontTouch/System/BluePrint/GameSystem/audiomanager.audiomanager_C"))
    (Default|Audiochange _returnvalue_2)))

(event Collision|EventActorBeginOverlap
  (params (OtherActor :type Actor%20Object%20Reference))
  ;[1 1 1] プログラムまとめた
)

(event Game|Damage|EventPointDamage
  (params (Damage :type Float%20%28single-precision%29) (DamageType :type Damage%20Type%20Object%20Reference) (HitLocation :type Vector :default "0, 0, 0") (HitNormal :type Vector :default "0, 0, 0") (HitComponent :type Primitive%20Component%20Object%20Reference) (BoneName :type Name :default "None") (ShotFromDirection :type Vector :default "0, 0, 0") (InstigatedBy :type Controller%20Object%20Reference) (DamageCauser :type Actor%20Object%20Reference) (HitInfo :type Hit%20Result%20Structure%20%28by%20ref%29))
  (Variables|Default|Setimpact HitNormal))

(fn ConstructionScript)

(fn Gotgravit
  (if (not (AI|Components|NavMovement|IsFalling (Variables|Character|GetCharacterMovement)))
    (if (Variables|Default|Getgravit)
      (Game|Damage|ApplyDamage self 3e+02 0 0)
      (Variables|Default|Setgravit false))))

(fn Timecontrol
  (bind _returnvalue (Utilities|Time|GetWorldDeltaSeconds))
  (bind _customtimedilation (Variables|Default|GetCustomTimeDilation))
  (bind _reverseactor (Variables|Default|Getreverseactor))
  (bind _returnvalue_2 (* _returnvalue 6e+01))
  (bind _returnvalue_3 (== _customtimedilation 1.0))
  (Utilities|FlowControl|Sequence
    (:then_0
      (Utilities|IsValid _reverseactor
        (:Is%20Valid
          (Default|Recordvalue _reverseactor (Variables|Default|GetHP) (Variables|/Script/Engine.MovementComponent|GetVelocity (Variables|Character|GetCharacterMovement)) false (Variables|Default|Getmytime))
          (Variables|Default|Settimecontroled (not _returnvalue_3))
          (Rendering|SetCustomDepthStencilValue (Variables|Character|GetMesh) (Math|Integer|SelectInt 1 3 _returnvalue_3))
          (if _returnvalue_3
            _))))
    (:then_1
      (Variables|Default|SetMutekiDamageTimer (- (Variables|Default|GetMutekiDamageTimer) _returnvalue_2))
      (Variables|Default|SetAACoolTime (- (Variables|Default|GetAACoolTime) _returnvalue_2))
      (if (Variables|Default|GetIsDpsCheckNow)
        (bind _output_get (Variables|Default|SetDpscheckTime (- (Variables|Default|GetDpscheckTime) _returnvalue)))
        (if (<= _output_get 0.0)
          (CallFunction|TimeIsOver))))))

(fn CCControl
  (Variables|/Script/Engine.CharacterMovementComponent|SetMaxWalkSpeed (Variables|Character|GetCharacterMovement) (Math|Float|SelectFloat (Variables|Default|Getwalkspeed) 0.0 (Variables|Default|Getcanwalk))))

(fn Moving)

(fn Gotdamage
  (params (NewParam :type Vector) (cause :type Actor%20Object%20Reference))
  (if (<= (Variables|Default|GetMutekiDamageTimer) 0.0)
    (if (< (Math|Vector|DotProduct (Math|Vector|Normalize (- NewParam (Transformation|GetActorLocation))) (Transformation|GetActorForwardVector)) -0.75)
      (Variables|Default|Setdamagegain (* (Variables|Default|Getdamagegain) 1.5)))
    (if (<= (Math|Random|RandomFloatinRange 0.0 1e+02) 5.0)
      (LocalVariables|Setcriticalhit true)
      (Variables|Default|Setdamagegain (* (Variables|Default|Getdamagegain) 2.0)))
    (Variables|Default|Setdamagegain (* (Variables|Default|Getdamagegain) (Math|Float|SelectFloat 1.0 1.5 (Variables|Default|GetHardMode))))
    (bind _returnvalue (UserInterface|CreateWidget "/Game/DontTouch/System/Widget/Ensyutu/damage.damage_C" 0 (Utilities|String|ToString(Integer) (Math|Float|Truncate (Variables|Default|Getdamagegain))) (LocalVariables|Getcriticalhit) (Math|Vector|SelectVector (Transformation|GetActorLocation) (Variables|Default|Getdaamgehitlocation) (Variables|Default|GetDamagetextOnEnemyActor))))
    (UserInterface|Viewport|AddtoViewport _returnvalue 0)
    (if (Variables|Default|GetIsDpsCheckNow)
      (Variables|Default|SetDpsCheckValue (- (Variables|Default|GetDpsCheckValue) (Variables|Default|Getdamagegain)))
      (else
        (Variables|Default|SetHP (- (Variables|Default|GetHP) (Variables|Default|Getdamagegain)))))
    (Animation|StopAnimMontage (Variables|Default|GetNormalAttackMotion))
    (Variables|Default|SetAACoolTime 3e+01)
    (Variables|Default|SetMutekiDamageTimer (Variables|Default|GetDefualtMutekiTimer))
    (Class|Message|ComboAdded(Message) cause (Variables|Default|GetAddScore) true)
    (Variables|Default|SetAddScore 0.0)
    (if (<= (Variables|Default|GetDpsCheckValue) 0.0)
      (if (Variables|Default|GetIsDpsCheckNow)
        (CallFunction|DpsCheckClear)))))

(fn Attackhantei
  (bind _attackedactor (Variables|Default|Getattackedactor))
  (Utilities|FlowControl|Sequence
    (:then_0
      (if (Variables|Default|Getcanapplydamage)
        (for _array_element (Collision|GetOverlappingActors (Variables|Default|GetBox) "/Game/DontTouch/player.player_C" :!class /Script/Engine.PrimitiveComponent)
          (if (not (Utilities|Array|ContainsItem _attackedactor _array_element))
            (Game|Damage|ApplyDamage _array_element (Variables|Default|GetATK) 0 self)
            (Utilities|Array|Add _attackedactor _array_element)))))
    (:then_1
      (if (<= (Math|Vector|Distance(Vector) (Transformation|GetActorLocation) (Transformation|GetActorLocation (Game|GetPlayerCharacter 0))) (Variables|Default|GetAttackRange))
        (CallFunction|AttackAnimation)))))

(fn Spawnmyspawner
  (bind _returnvalue (Game|SpawnActorfromClass "/Game/DontTouch/JuyouBluePrint/SpawnerFold/spawner.spawner_C" (Transformation|GetActorTransform) "AlwaysSpawn" 0 false 0))
  (Variables|Default|Setmycreatedspawner _returnvalue)
  (Default|Onlyspawn _returnvalue))

(fn TasizanSuruKansuu
  (for _array_element (Variables|Default|Getsaveddamage)
    (LocalVariables|SetAdded (+ _array_element (LocalVariables|GetAdded))))
  (return (LocalVariables|GetAdded)))

(event EventReverseValue
  (params (HP :type Float%20%28double-precision%29) (Velocity :type Vector :default "0, 0, 0") (time :type Float%20%28double-precision%29))
  (Variables|Default|SetHP HP)
  (Variables|/Script/Engine.MovementComponent|SetVelocity (Variables|Character|GetCharacterMovement) Velocity)
  (Variables|Default|Setmytime time))

(event EventSetnewcustomtime
  (params (dilution :type Float%20%28double-precision%29) (time :type Float%20%28double-precision%29) (isrewind :type Boolean))
  (bind _reverseactor (Variables|Default|Getreverseactor))
  (Utilities|IsValid _reverseactor
    (:Is%20Valid
      (Default|Settimedictiom _reverseactor dilution time isrewind))))

(event OnSeePawn(PawnSensing)
  (params (Pawn :type Pawn%20Object%20Reference))
  (if (Variables|Default|Getboss)
    (CallFunction|IamSeeing)))

(event Custom|IamSeeing
  (Utilities|FlowControl|DoOnce false
    (:Completed
      (CallFunction|Start)
      (bind _returnvalue (UserInterface|CreateWidget "/Game/DontTouch/System/Widget/System/caution.caution_C" 0 false (Variables|Default|Getname) self true))
      (Variables|Default|SetMyCaution _returnvalue)
      (UserInterface|Viewport|AddtoViewport _returnvalue 0)
      (bind _returnvalue_2 (Actor|GetActorOfClass "/Game/DontTouch/System/BluePrint/GameSystem/audiomanager.audiomanager_C"))
      (Default|Audiochange _returnvalue_2))))

(event Custom|AttackAnimation
  (bind _mesh (Variables|Character|GetMesh))
  (bind _returnvalue (Components|SkeletalMesh|GetAnimInstance _mesh))
  ;[1 1 1] 攻撃系
  (Utilities|IsValid _mesh
    (:Is%20Valid
      (Utilities|IsValid _returnvalue
        (:Is%20Valid
          (if (not (Animation|Montage|MontageIsPlaying _returnvalue 0))
            (if (Variables|Default|Getcanwalk)
              (if (<= (Variables|Default|GetAACoolTime) 0.0)
                (Animation|PlayAnimMontage (Variables|Default|GetNormalAttackMotion) 1.0 "None")))))))))

(event Custom|autoattack)

(event Custom|attackon
  ;[1 1 1] 攻撃系
  (Variables|Default|Setcanapplydamage true)
  (Utilities|Array|Clear (Variables|Default|Getattackedactor)))

(event Custom|AttackOff
  ;[1 1 1] 攻撃系
  (Variables|Default|Setcanapplydamage false))

(event Custom|applytimedamage
  (if (Variables|Default|Gettimecontroled)
    (goto _label Reset)
    (else
      (Utilities|FlowControl|DoOnce false :!label _label
        (:Completed
          (bind _added1 (CallFunction|TasizanSuruKansuu))
          (Game|Damage|ApplyDamage self _added1 0 (Game|GetPlayerCharacter 0) "/Script/Engine.DamageType")
          (Utilities|Array|Clear (Variables|Default|Getsaveddamage)))))))

(event Game|Damage|EventAnyDamage
  (params (Damage :type Float%20%28single-precision%29) (DamageType :type Damage%20Type%20Object%20Reference) (InstigatedBy :type Controller%20Object%20Reference) (DamageCauser :type Actor%20Object%20Reference))
  (bind _returnvalue (Transformation|GetActorLocation))
  (bind _returnvalue_2 (Transformation|GetActorLocation DamageCauser))
  (bind _mesh (Variables|Character|GetMesh))
  (bind _reverseactor (Variables|Default|Getreverseactor))
  (bind _mycreatedspawner (Variables|Default|Getmycreatedspawner))
  (Variables|Default|Setdamagegain Damage)
  (Utilities|FlowControl|Sequence
    (:then_0
      (Utilities|IsValid DamageCauser
        (:Is%20Valid
          (CallFunction|Gotdamage _returnvalue_2 DamageCauser)
          (if (<= (Variables|Default|GetHP) 0.0)
            (Utilities|FlowControl|DoOnce false
              (:Completed
                (CallFunction|Died)
                (Class|Message|Kyoukichange(Message) (Game|GetPlayerCharacter 0) (Math|Float|SelectFloat 4e+01 1.0 (Variables|Default|Getisally)))
                (Utilities|FlowControl|Delay 0.2)
                (Actor|Tick|SetActorTickEnabled false)
                (Physics|SetSimulatePhysics _mesh true)
                (Physics|AddImpulse _mesh (* (Variables|Default|Getimpact) -4000) "None" false)
                (Collision|SetCollisionEnabled (Variables|Collision|GetCapsuleComponent) "NoCollision")
                (Pawn|Components|CharacterMovement|SetMovementMode (Variables|Character|GetCharacterMovement) "MOVE_None" 0)
                (Utilities|FlowControl|Sequence
                  (:then_0
                    (Utilities|IsValid _reverseactor
                      (:Is%20Valid
                        (Actor|DestroyActor _reverseactor)
                        (bind _asai (Utilities|Casting|CastToai (Pawn|GetController))
                          (:then
                            (Default|Logicstart _asai false))
                          (:CastFailed
                            _)))
                      (:Is%20Not%20Valid
                        _))
                    (Utilities|FlowControl|Delay 1.0)
                    (Niagara|SpawnSystematLocation "/Game/DontTouch/Effect/death.death" (Transformation|GetSocketLocation (Variables|Character|GetMesh) "Spine_02"))
                    (Utilities|IsValid _mycreatedspawner
                      (:Is%20Valid
                        (Actor|DestroyActor _mycreatedspawner))
                      (:Is%20Not%20Valid
                        _))
                    (Actor|DestroyActor)))))))))
    (:then_1
      (Utilities|IsValid DamageCauser
        (:Is%20Valid
          (Niagara|SpawnSystematLocation "/Game/DontTouch/Effect/bisya.bisya" _returnvalue (Math|Rotator|FindLookatRotation _returnvalue_2 _returnvalue)))))
    (:then_2
      (if (== (Utilities|GetClass DamageType) "/Game/DontTouch/System/BluePrint/tokitome.tokitome_C")
        (Math|Integer|IncrementInt (Variables|Default|Getdamagecombo))))))

(event EventDestroyed
  (bind _myspawner (Variables|Default|Getmyspawner))
  (Utilities|IsValid _myspawner
    (:Is%20Valid
      (Default|Enemykilled _myspawner))))

(event Custom|spawn
  (Actor|Tick|SetActorTickEnabled true)
  (Rendering|SetActorHiddenInGame false)
  (Collision|SetCollisionEnabled (Variables|Collision|GetCapsuleComponent) "QueryAndPhysics")
  (Collision|SetCollisionEnabled (Variables|Character|GetMesh) "QueryAndPhysics")
  (Class|Message|Logicstart(Message) (AI|GetAIController self) true)
  (CallFunction|Start))

(event Custom|start
  (Utilities|FlowControl|DoOnce false
    (:Completed
      (CallFunction|Spawn)
      (bind _returnvalue (Game|SpawnActorfromClass "/Game/DontTouch/JuyouBluePrint/reversingsystem.reversingsystem_C" (Transformation|GetActorTransform) "AlwaysSpawn" 0 0 self false 0))
      (Variables|Default|Setreverseactor _returnvalue)
      (Utilities|FlowControl|Delay 0.0)
      (Niagara|SpawnSystematLocation "/Game/DontTouch/Effect/spawn.spawn" (Transformation|GetActorLocation))
      (Utilities|FlowControl|Delay 0.3)
      (bind _returnvalue_2 (Niagara|SpawnSystematLocation "/Game/DontTouch/Effect/hate.hate" (Transformation|GetActorLocation)))
      (Effects|Components|ParticleSystem|SetVectorParameter _returnvalue_2 "target" (Transformation|GetActorLocation (Game|GetPlayerCharacter 0)))
      (Utilities|FlowControl|Delay (Math|Random|RandomFloatinRange 1.0 4.0)))))

(event EventBeginPlay
  (bind _asinstance (Utilities|Casting|CastToinstance (Game|GetGameInstance))
    (:then
      (Variables|Default|SetHardMode (Variables|/Game/DontTouch/System/BluePrint/GameSystem/instance.instance_C|GetHardMode _asinstance))
      (bind _output_get (Variables|Default|SetMaxDpsCheckValue (* (Variables|Default|GetMaxDpsCheckValue) (Math|Float|SelectFloat 1.2 1.0 (Variables|Default|GetHardMode)))))
      (Variables|Default|SetDpsCheckValue _output_get)
      (Utilities|Time|SetTimerbyFunctionName 0 "applytimedamage" 0.05 true)
      (Variables|Default|SetHP (Variables|Default|GetMaxHp))
      (if (not (Variables|Default|Getboss))
        (CallFunction|Spawn)
        (bind _returnvalue (Game|SpawnActorfromClass "/Game/DontTouch/JuyouBluePrint/reversingsystem.reversingsystem_C" (Transformation|GetActorTransform) "AlwaysSpawn" 0 0 self false 0))
        (Variables|Default|Setreverseactor _returnvalue)
        (Utilities|FlowControl|Delay 0.0)
        (Niagara|SpawnSystematLocation "/Game/DontTouch/Effect/spawn.spawn" (Transformation|GetActorLocation))
        (Utilities|FlowControl|Delay 0.3)
        (bind _returnvalue_2 (Niagara|SpawnSystematLocation "/Game/DontTouch/Effect/hate.hate" (Transformation|GetActorLocation)))
        (Effects|Components|ParticleSystem|SetVectorParameter _returnvalue_2 "target" (Transformation|GetActorLocation (Game|GetPlayerCharacter 0)))
        (Utilities|FlowControl|Delay (Math|Random|RandomFloatinRange 1.0 4.0))))
    (:CastFailed
      (CallFunction|Printlog "Instance not Found!!(Enemy/EventGraph/BeginPlayAndStart)" "NewEnumerator4" true 2.0 false "(R=0.000000,G=1.000000,B=0.956444,A=1.000000)"))))

(event EventHuttobasu
  (params (Vector :type Vector :default "0, 0, 0"))
  (bind _mesh (Variables|Character|GetMesh))
  (Physics|AddImpulse (Variables|Character|GetCharacterMovement) Vector true)
  (Utilities|FlowControl|Delay 0.05)
  (if (Physics|IsSimulatingPhysics _mesh "None")
    (Physics|AddImpulse _mesh Vector "None" true)))

(event Custom|DpsCheckClear
  (Variables|Default|SetIsDpsCheckNow false)
  (bind _returnvalue (UserInterface|CreateWidget "/Game/DontTouch/System/Widget/Ensyutu/DpsCheckIsComplete.DpsCheckIsComplete_C"))
  (UserInterface|Viewport|AddtoViewport _returnvalue 0)
  (for _index (range 0 6)
    (Niagara|SpawnSystematLocation "/Game/DontTouch/Effect/DPSBurst.DPSBurst" (+ (Transformation|GetActorLocation) (* (Math|Random|RandomUnitVector) 800)))))

(event Custom|DpsCheckIsStart
  (params (Notice :type Text) (ChargeText :type Text))
  (bind _returnvalue (UserInterface|CreateWidget "/Game/DontTouch/System/Widget/System/DPSCheck.DPSCheck_C" 0 self ChargeText))
  (UserInterface|Viewport|AddtoViewport _returnvalue 0)
  (bind _returnvalue_2 (UserInterface|CreateWidget "/Game/DontTouch/System/Widget/System/BattleNotice.BattleNotice_C" 0 Notice))
  (UserInterface|Viewport|AddtoViewport _returnvalue_2 0)
  (Variables|Default|SetIsDpsCheckIsDone true))

(event Custom|TimeIsOver
  (Variables|Default|SetIsDpsCheckIsDone true))

(event Custom|KnockUp
  (Variables|/Script/Engine.CharacterMovementComponent|SetGravityScale (Variables|Character|GetCharacterMovement) 0.05)
  (Utilities|FlowControl|Delay 2.0)
  (Variables|/Script/Engine.CharacterMovementComponent|SetGravityScale (Variables|Character|GetCharacterMovement) 1.0))

(event EventGoingDamage
  (params (damage :type Float%20%28double-precision%29) (hitlocation :type Vector :default "0, 0, 0") (iroiro :type Boolean) (Cause :type Actor%20Object%20Reference) (DamageType :type Damage%20Type%20Class%20Reference) (DamageScore :type Float%20%28double-precision%29) (AdditonalEffect :type AdditionalEffect%20Enum :default "NewEnumerator3") (AdditionalEffectTime :type Float%20%28double-precision%29) (GoingStun :type Float%20%28double-precision%29))
  (if (Utilities|Enum|Equal(Enum) AdditonalEffect "NewEnumerator0")
    (CallFunction|KnockUp))
  (|GoingDamaged damage damage Cause DamageType hitlocation DamageScore))

(event EventTick
  (params (DeltaSeconds :type Float%20%28single-precision%29))
  ;[1 1 1] Tick
  (CallFunction|Timecontrol)
  (CallFunction|CCControl)
  (CallFunction|Attackhantei))

(event Custom|talk
  (params (text :type Text) (talker :type Text) (anim :type textanim%20Enum :default "NewEnumerator0") (rotating :type Float%20%28double-precision%29))
  (|TalkingMethod anim rotating talker text))